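; Behavior tree service for the Stoopid turret AI that acquires an enemy target within the turret's range.
; On search start it waits briefly, keeping the current target if still in the cached overlap list and alive.
; Otherwise it sphere-overlaps, picks a random actor and rejects same-team picks via BPC_Team, retrying once after a delay.
; The result sets or clears the turret's AITarget and blackboard keys, without any line-of-sight trace.
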(event EventReceiveSearchStart
  (params (OwnerActor :type Actor%20Object%20Reference))
  ;[0.5569 0.5569 0.5569] Check AI Consinsus for AI location
  (Utilities|FlowControl|Sequence
    (:then_0
      ;;[0.0875 0.1235 0.4375] Set controller referance
      (Utilities|FlowControl|DoOnce false
        (:Completed
          (bind _asbp_ai_turret_controller (Utilities|Casting|CastToBP_AI_Turret_Controller OwnerActor))
          (Variables|Default|SetBSP_Shooter_AIControllerRef _asbp_ai_turret_controller))))
    (:then_1
      ;;[0.0875 0.1235 0.4375] Check AI Target is still valid if it is then Bypass the rest of the detection process
      (Utilities|FlowControl|Delay 1.0)
      (Utilities|IsValid (Variables|/Game/BSP_StoopidAI/BSP_StoopidTurret/Blueprints/Characters/StoopidTurret/BP_StoopidTurret_Parent.BP_StoopidTurret_Parent_C|GetAITarget (CallFunction|FBSPGetStoopidTurretParent))
        (:Is%20Valid
          (if (not (and (Utilities|Array|ContainsItem (Variables|Default|GetBSP_Shooter_ActorsCurrentlyInSphere) (Variables|/Game/BSP_StoopidAI/BSP_StoopidTurret/Blueprints/Characters/StoopidTurret/BP_StoopidTurret_Parent.BP_StoopidTurret_Parent_C|GetAITarget (CallFunction|FBSPGetStoopidTurretParent))) (not (Variables|/Game/BSP_StoopidAI/Shared/Component/BPC_Team.BPC_Team_C|GetIsDead (Actor|GetComponentbyClass (Variables|/Game/BSP_StoopidAI/BSP_StoopidTurret/Blueprints/Characters/StoopidTurret/BP_StoopidTurret_Parent.BP_StoopidTurret_Parent_C|GetAITarget (CallFunction|FBSPGetStoopidTurretParent)) "/Game/BSP_StoopidAI/Shared/Component/BPC_Team.BPC_Team_C")))))
            ;;[0.0875 0.1235 0.4375] get location and Sphere overlaps
            (Variables|Default|SetBSP_Shooter_CurrentLocation (Transformation|GetActorLocation (Pawn|GetControlledPawn (Variables|Default|GetBSP_Shooter_AIControllerRef))) :!label _label)
            (bind _outactors (Collision|SphereOverlapActors (Transformation|GetActorLocation (Pawn|GetControlledPawn (Variables|Default|GetBSP_Shooter_AIControllerRef))) (Variables|/Game/BSP_StoopidAI/BSP_StoopidTurret/Blueprints/PrimaryDataAssets/BP_PDA_TurretType.BP_PDA_TurretType_C|GetRange (Variables|/Game/BSP_StoopidAI/BSP_StoopidTurret/Blueprints/Characters/StoopidTurret/BP_StoopidTurret_Parent.BP_StoopidTurret_Parent_C|GetTurret_Data (CallFunction|FBSPGetStoopidTurretParent))) (Variables|Default|GetBSP_Shooter_DesiredTargetTypes) 0 (Utilities|Array|MakeArray (Pawn|GetControlledPawn (Variables|Default|GetBSP_Shooter_AIControllerRef)))))
            (Variables|Default|SetBSP_Shooter_ActorsCurrentlyInSphere _outactors)
            ;;[0.0875 0.1235 0.4375] Check Validity of the actor
            (bind _outitem (CallFunction|FBSPRandomActorwithinRange :!label _label_2))
            (Utilities|MValidateRandomActor _outitem
              (:SameTeam
                (if (Variables|Default|GetLoopBreaker)
                  (Utilities|Array|Clear (Variables|Default|GetBSP_Shooter_SphereTemp))
                  (Variables|Default|SetLoopBreaker false)
                  (Utilities|Array|Clear (Variables|Default|GetBSP_Shooter_SphereTemp))
                  (Utilities|Array|Clear (Variables|Default|GetBSP_Shooter_ActorsCurrentlyInSphere))
                  (Variables|Default|SetBSP_Shooter_ActorInVisabilitySphere 0)
                  ;;[0.0875 0.1235 0.4375] Nulify All Values
                  (Variables|/Game/BSP_StoopidAI/BSP_StoopidTurret/Blueprints/Characters/StoopidTurret/BP_StoopidTurret_Parent.BP_StoopidTurret_Parent_C|SetAITarget (CallFunction|FBSPGetStoopidTurretParent) 0 :!label _label_3)
                  (Class|BTFunctionLibrary|ClearBlackboardValue (Variables|Default|GetBSP_Shooter_AITarget))
                  (Class|BTFunctionLibrary|ClearBlackboardValue (Variables|Default|GetBSP_Shooter_TargetLocation))
                  (else
                    (Utilities|FlowControl|Delay 0.2)
                    (Variables|Default|SetLoopBreaker true)
                    (goto _label_2))))
              (:NulValue
                (goto _label_3))
              (:Valid
                (Variables|Default|SetBSP_Shooter_ActorInVisabilitySphere _outitem)
                ;;[0.0875 0.1235 0.4375] Set Blackboard Values
                (Variables|/Game/BSP_StoopidAI/BSP_StoopidTurret/Blueprints/Characters/StoopidTurret/BP_StoopidTurret_Parent.BP_StoopidTurret_Parent_C|SetAITarget (CallFunction|FBSPGetStoopidTurretParent) (Variables|Default|GetBSP_Shooter_ActorInVisabilitySphere))
                (Class|BTFunctionLibrary|SetBlackboardValueasObject (Variables|Default|GetBSP_Shooter_AITarget) (Variables|Default|GetBSP_Shooter_ActorInVisabilitySphere))
                (AI|BehaviorTree|SetBlackboardValueasVector (Variables|Default|GetBSP_Shooter_TargetLocation) (Transformation|GetActorLocation (Variables|Default|GetBSP_Shooter_ActorInVisabilitySphere)))))))
        (:Is%20Not%20Valid
          (goto _label))))))

(fn FBSPActorinSameTeam
  (params (InputPin :type Actor%20Object%20Reference))
  (bind (_resultinvalid _bsp_team) (CallFunction|FBSPGetOwnerTeam))
  (bind _returnvalue (Actor|GetComponentbyClass InputPin "/Game/BSP_StoopidAI/Shared/Component/BPC_Team.BPC_Team_C"))
  ;[0.07451 0.1216 0.2706] Check target and owner to confirm the team is not the same
  (Utilities|IsValid InputPin
    (:Is%20Valid
      (if _resultinvalid
        (return true)
        (else
          (Utilities|IsValid _returnvalue
            (:Is%20Valid
              (if (Utilities|Enum|Equal(Enum) _bsp_team (Variables|/Game/BSP_StoopidAI/Shared/Component/BPC_Team.BPC_Team_C|GetBSP_Team _returnvalue))
                (return true)
                (else
                  _)))
            (:Is%20Not%20Valid
              _))
          (return false))))
    (:Is%20Not%20Valid
      (return true))))

(fn FBSPGetOwnerTeam
  (bind _bsp_shooter_aicontrollerref (Variables|Default|GetBSP_Shooter_AIControllerRef))
  (bind _returnvalue (Pawn|GetControlledPawn _bsp_shooter_aicontrollerref))
  (bind _returnvalue_2 (Actor|GetComponentbyClass _returnvalue "/Game/BSP_StoopidAI/Shared/Component/BPC_Team.BPC_Team_C"))
  ;[0.07451 0.1216 0.2706] Check Ai controller reference and confirm value of team
  (Utilities|IsValid _returnvalue_2
    (:Is%20Valid
      (return false (Variables|/Game/BSP_StoopidAI/Shared/Component/BPC_Team.BPC_Team_C|GetBSP_Team _returnvalue_2)))
    (:Is%20Not%20Valid
      (return true "NewEnumerator4"))))

(fn FBSPRandomActorwithinRange
  (bind _bsp_shooter_actorscurrentlyinsphere (Variables|Default|GetBSP_Shooter_ActorsCurrentlyInSphere))
  ;[0.0875 0.1235 0.4375] Get Random actor from Array
  (if (Utilities|Array|IsValidIndex _bsp_shooter_actorscurrentlyinsphere)
    (return (.OutItem (Utilities|Array|Random _bsp_shooter_actorscurrentlyinsphere)))))

(fn FBSPGetStoopidTurretParent
  ;[0.0875 0.1235 0.4375] Get Turrent Parent from AI controller
  (return (.AsBP%20Stoopid%20Turret%20Parent (Utilities|Casting|CastToBP_StoopidTurret_Parent (Variables|/Script/Engine.Actor|GetInstigator (Variables|Default|GetBSP_Shooter_AIControllerRef))))))