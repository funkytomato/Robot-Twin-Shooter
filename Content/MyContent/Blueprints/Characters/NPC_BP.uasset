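; NPC character Blueprint that handles health, damage reactions, death and shooting state.
; BeginPlay caches its NPC_AnimBP instance and NPC_AIController_BP.
; AnyDamage subtracts health, playing a montage while alive; at zero it ragdolls the mesh, stops AI brain logic, disables capsule collision and stops shooting.
; StartShooting and StopShooting only set IsShooting flags on the character and anim instance, with no firing logic here.
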(event Custom|StartShooting
  ;[1 1 1] Shooting
  (Variables|/Game/MyContent/Blueprints/Characters/NPC_AnimBP.NPC_AnimBP_C|SetIsShooting? (Variables|Default|GetAnimInstance) true)
  (Variables|Default|SetIsShooting true))

(event Custom|StopShooting
  ;[1 1 1] Shooting
  (Variables|/Game/MyContent/Blueprints/Characters/NPC_AnimBP.NPC_AnimBP_C|SetIsShooting? (Variables|Default|GetAnimInstance) false)
  (Variables|Default|SetIsShooting false))

(event EventBeginPlay
  ;[1 1 1] BeginPlay - Get references to Animation Instance and AIController
  (Utilities|FlowControl|Sequence
    (:then_0
      (bind _asnpc_anim_bp (Utilities|Casting|CastToNPC_AnimBP (Components|SkeletalMesh|GetAnimInstance (Variables|Character|GetMesh))))
      (Variables|Default|SetAnimInstance _asnpc_anim_bp))
    (:then_1
      (bind _asnpc_aicontroller_bp (Utilities|Casting|CastToNPC_AIController_BP (AI|GetAIController self)))
      (Variables|Default|SetPawnAIController _asnpc_aicontroller_bp))))

(event Game|Damage|EventAnyDamage
  (params (Damage :type Float%20%28single-precision%29) (DamageType :type Damage%20Type%20Object%20Reference) (InstigatedBy :type Controller%20Object%20Reference) (DamageCauser :type Actor%20Object%20Reference))
  ;[1 1 1] AnyDamage
  (bind _output_get (Variables|Default|SetHealth (- (Variables|Default|GetHealth) Damage)))
  (if (<= _output_get 0.0)
    (Physics|SetSimulatePhysics (Variables|Character|GetMesh) true)
    (AI|Logic|StopLogic (Variables|/Script/AIModule.AIController|GetBrainComponent (AI|GetAIController self)) "")
    (Collision|SetCollisionEnabled (Variables|Collision|GetCapsuleComponent) "NoCollision")
    (CallFunction|StopShooting)
    (else
      (Animation|Montage|MontagePlay (Variables|Default|GetAnimInstance) 0 1.0 "MontageLength" 0.0 true))))

(fn ConstructionScript)