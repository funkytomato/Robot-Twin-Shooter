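; Interactable computer that can start contaminated by a virus and tracks clamped health, which sets whether it is functioning.
; When contaminated, a looping timer plays a timeline that wobbles the mesh, and a dynamic material is created.
; Interacting first clears contamination, then later interactions add health, stopping the wobble at full health.
; The contamination colour event is empty, and the emissive colour logic is disconnected.
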(event Custom|ContaminatedEffects
  (bind _returnvalue (Transformation|GetActorLocation))
  (bind _returnvalue_2 (Transformation|GetActorRotation))
  (bind _interactablemesh (Variables|Default|GetInteractableMesh))
  ;[1 1 1] Apply Contamination effects, make mesh rock/wobble about, and stop
  (bind (_direction _wobble) (Timeline|WobbleTimeline Play)
    (:Update
      (switch Utilities|FlowControl|Switch|SwitchonETimelineDirection _direction
        (:Forward
          (Transformation|SetWorldRotation _interactablemesh (Math|Rotator|Lerp(Rotator) (Transformation|GetActorRotation) (Math|Rotator|MakeRotator (+ (.roll _returnvalue_2) 0.0) (+ (.pitch _returnvalue_2) 0.0) (+ (.yaw _returnvalue_2) 45.0)) _wobble) false false)
          (Transformation|SetWorldLocation _interactablemesh (Math|Vector|Lerp(Vector) (Transformation|GetActorLocation) (Math|Vector|MakeVector (.x _returnvalue) (.y _returnvalue) (- (.z _returnvalue) 2.0)) _wobble) false false))))))

(event Custom|StopContaminatedEffects
  (bind _returnvalue (Transformation|GetActorLocation))
  (bind _returnvalue_2 (Transformation|GetActorRotation))
  (bind _interactablemesh (Variables|Default|GetInteractableMesh))
  ;[1 1 1] Apply Contamination effects, make mesh rock/wobble about, and stop
  (Utilities|Time|ClearandInvalidateTimerbyHandle (Variables|Default|GetWobbleTimerRef))
  (Development|PrintString "HeUncontaminated")
  (bind (_direction _wobble) (Timeline|WobbleTimeline Stop)
    (:Update
      (switch Utilities|FlowControl|Switch|SwitchonETimelineDirection _direction
        (:Forward
          (Transformation|SetWorldRotation _interactablemesh (Math|Rotator|Lerp(Rotator) (Transformation|GetActorRotation) (Math|Rotator|MakeRotator (+ (.roll _returnvalue_2) 0.0) (+ (.pitch _returnvalue_2) 0.0) (+ (.yaw _returnvalue_2) 45.0)) _wobble) false false)
          (Transformation|SetWorldLocation _interactablemesh (Math|Vector|Lerp(Vector) (Transformation|GetActorLocation) (Math|Vector|MakeVector (.x _returnvalue) (.y _returnvalue) (- (.z _returnvalue) 2.0)) _wobble) false false))))))

(event Custom|ApplyBadColour)

(event EventInteract
  (params (amount :type Float%20%28single-precision%29))
  ;[1 1 1] Player Interaction, cure virus, give health and stop contamination effects
  (|CallParentFunction amount)
  (if (Variables|Default|GetIsContaminated?)
    ;;[1 1 1] Reacquire Computer, remove virus
    (Variables|Default|SetIsContaminated? false)
    (else
      ;;[1 1 1] Not contaminated, increase health of computer
      (CallFunction|IncreaseHealth amount)
      (if (>= (Variables|Default|GetHealth) 1e+02)
        (CallFunction|StopContaminatedEffects)))))

(event EventBeginPlay
  (bind _interactablemesh (Variables|Default|GetInteractableMesh))
  ;[1 1 1] On BeginPlay, start Contaminated Effects if contaminated
  (if (Variables|Default|GetIsContaminated?)
    (bind _returnvalue (Utilities|Time|SetTimerbyFunctionName 0 "ContaminatedEffects" 1.0 true))
    (Variables|Default|SetWobbleTimerRef _returnvalue)
    (bind _returnvalue_2 (Rendering|Material|CreateDynamicMaterialInstance _interactablemesh 0 "/Game/SciFi_Props/Materials/MI_Box_8.MI_Box_8" "None" :!class /Script/Engine.PrimitiveComponent))
    (bind _output_get (Variables|Default|SetMyDynamicMaterial _returnvalue_2))
    (Rendering|Material|SetMaterial _interactablemesh 0 _output_get)
    (CallFunction|ApplyBadColour)))

(fn ConstructionScript
  (|CallParentFunction))

(fn IncreaseHealth
  (params (amount :type Float%20%28single-precision%29))
  (bind _output_get (Variables|Default|SetHealth (Math|Float|Clamp(Float) (+ (Variables|Default|GetHealth) amount) 0.0 1e+02)))
  (Variables|Default|SetIsFunctioning? (> _output_get 0.0)))

(fn DecreaseHealth
  (params (amount :type Float%20%28single-precision%29))
  (bind _output_get (Variables|Default|SetHealth (Math|Float|Clamp(Float) (- (Variables|Default|GetHealth) amount) 0.0 1e+02)))
  (Variables|Default|SetIsFunctioning? (> _output_get 0.0)))